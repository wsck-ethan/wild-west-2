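; BP_AIShooting is an actor that acts as a gun pickup for BP_ThirdPersonCharacter and also damages that character on contact.
; Overlapping Collision snaps the Cylinder component to the character mesh's Gun socket, enables CanShoot and shows the crosshair.
; Overlapping the separate DamageCollision subtracts Damage directly from the character's Health3dPerson.
; Despite the name, the graph contains no AI or firing logic.
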(event OnComponentBeginOverlap(collision)
  (params (OverlappedComponent :type Primitive%20Component%20Object%20Reference) (OtherActor :type Actor%20Object%20Reference) (OtherComp :type Primitive%20Component%20Object%20Reference) (OtherBodyIndex :type Integer) (bFromSweep :type Boolean) (SweepResult :type Hit%20Result%20Structure%20%28by%20ref%29))
  (bind _asbp_third_person_character (Utilities|Casting|CastToBP_ThirdPersonCharacter OtherActor))
  (Transformation|AttachComponentToComponent (Variables|Default|GetCylinder) (Variables|/Script/Engine.Character|GetMesh _asbp_third_person_character) "Gun" "SnapToTarget" "SnapToTarget" "SnapToTarget" true)
  (Variables|/Game/ThirdPerson/Blueprints/BP_ThirdPersonCharacter.BP_ThirdPersonCharacter_C|SetCanShoot _asbp_third_person_character true)
  (Default|ShowCrosshair _asbp_third_person_character))

(event OnComponentBeginOverlap(DamageCollision)
  (params (OverlappedComponent :type Primitive%20Component%20Object%20Reference) (OtherActor :type Actor%20Object%20Reference) (OtherComp :type Primitive%20Component%20Object%20Reference) (OtherBodyIndex :type Integer) (bFromSweep :type Boolean) (SweepResult :type Hit%20Result%20Structure%20%28by%20ref%29))
  (bind _asbp_third_person_character (Utilities|Casting|CastToBP_ThirdPersonCharacter OtherActor))
  (Variables|/Game/ThirdPerson/Blueprints/BP_ThirdPersonCharacter.BP_ThirdPersonCharacter_C|SetHealth%203d%20person _asbp_third_person_character (- (Variables|/Game/ThirdPerson/Blueprints/BP_ThirdPersonCharacter.BP_ThirdPersonCharacter_C|GetHealth%203d%20person _asbp_third_person_character) (Variables|Default|GetDamage))))

(fn ConstructionScript)