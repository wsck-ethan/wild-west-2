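; BP_Ranged_Enemy is a gun-carrying enemy that arms itself when play begins.
; After the parent BeginPlay, EquipWeopon spawns a BP_gun, stores it as WeaponActor and attaches it to the mesh's GunSocket.
; It saves the attach result in IsWeldingWeopon, then calls the OnweoponEquiped dispatcher.
; No AI, firing or tick logic is defined in this Blueprint itself.
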(event EventBeginPlay
  (|CallParentFunction)
  (CallFunction|EquipWeopon))

(event Collision|EventActorBeginOverlap
  (params (OtherActor :type Actor%20Object%20Reference)))

(event EventTick
  (params (DeltaSeconds :type Float%20%28single-precision%29)))

(event EventEquipWeopon
  (bind _returnvalue (Game|SpawnActorfromClass "/Game/WildWest/weopons/BP_gun.BP_gun_C" (Math|Transform|MakeTransform "0, 0, 0") "Undefined" "MultiplyWithRoot" 0 0))
  (bind _output_get (Variables|Default|SetweaponActor _returnvalue))
  (bind _returnvalue_2 (Transformation|AttachComponentToComponent _output_get (Variables|Character|GetMesh) "GunSocket" "KeepRelative" "KeepRelative" "KeepRelative" true))
  (Variables|Default|Setis%20welding%20weopon _returnvalue_2)
  (Default|CallOnweoponEquiped))

(fn ConstructionScript
  (|CallParentFunction))