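; Base AI character Blueprint for the WildWest game, providing patrol route access, movement speed presets, weapon equipping, attacking and health.
; Attack plays a montage on the mesh and fires an OnAttackEnd dispatcher, with a placeholder delay standing in until a montage is set.
; Equipping spawns a gun attached to the R_Gun socket.
; Overlaps from AI-damage projectiles on the damage collision reduce health, destroying the actor at zero.
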(event OnComponentBeginOverlap(DamageCollison)
  (params (OverlappedComponent :type Primitive%20Component%20Object%20Reference) (OtherActor :type Actor%20Object%20Reference) (OtherComp :type Primitive%20Component%20Object%20Reference) (OtherBodyIndex :type Integer) (bFromSweep :type Boolean) (SweepResult :type Hit%20Result%20Structure%20%28by%20ref%29))
  (bind _asbp_projectile_aidamage (Utilities|Casting|CastToBP_Projectile_AIDamage OtherActor)
    (:then
      (bind _output_get (Variables|Default|Sethealth (- (Variables|Default|Gethealth) (Variables|/Game/WildWest/Ralph_Young/BP_Projectile_AIDamage.BP_Projectile_AIDamage_C|GetDamage _asbp_projectile_aidamage))))
      (if (<= _output_get 0)
        (Actor|DestroyActor)))
    (:CastFailed
      (Development|PrintString "Hello"))))

(event Custom|weld%20weopon
  (bind _returnvalue (Game|SpawnActorfromClass "/Game/WildWest/weopons/BP_gun.BP_gun_C" (Transformation|GetActorTransform) "Undefined" "MultiplyWithRoot" 0 0))
  (Transformation|AttachComponentToComponent _returnvalue (Variables|Character|GetMesh) "R_Gun" "SnapToTarget" "SnapToTarget" "SnapToTarget" true)
  (Variables|Default|Setis%20welding%20weopon true))

(event Custom|attack
  (Animation|Montage|PlayMontage (Variables|Character|GetMesh) 0
    (:then
      ;[1 1 1] delete when montage play is set
      (Utilities|FlowControl|Delay 5.0))
    (:OnCompleted
      _)
    (:OnInterrupted
      _))
  (Default|CallOnAttackEnd))

(event EventBeginPlay)

(fn ConstructionScript)

(fn GetPatrolRoute
  (return (Variables|AI|GetPatrolRoute)))

(fn SetMovementSpeed
  (params (speed :type E_movementSpeed%20Enum :default "NewEnumerator0"))
  (bind _output_get (Variables|/Script/Engine.CharacterMovementComponent|SetMaxWalkSpeed (Variables|Character|GetCharacterMovement) (Utilities|Select :Index speed :NewEnumerator0 0.0 :NewEnumerator1 1e+02 :NewEnumerator2 3e+02 :NewEnumerator3 5e+02)))
  (return _output_get))