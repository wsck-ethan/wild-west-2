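; BP_patrol_route is a patrol path for AI, built on a spline whose points serve as waypoints.
; IncrementPatrolRoute steps PatrolIndex by Direction and flips Direction at the first and last points, so the route runs back and forth instead of looping.
; GetSplinePointWorldLocation returns the world location of the current point.
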(event Custom|IncrementPatrolRoute
  (bind _output_get (Variables|Default|SetpatrolIndex (+ (Variables|Default|GetpatrolIndex) (Variables|Default|Getdirection))))
  (if (== _output_get (- (Spline|GetNumberOfSplinePoints (Variables|Default|GetPatrolRoute)) 1))
    (Variables|Default|Setdirection -1)
    (elif (== (Variables|Default|GetpatrolIndex) 0)
      (Variables|Default|Setdirection 1))))

(fn ConstructionScript)

(fn GetSplinePointWorldLocation
  (return (Spline|GetLocationatSplinePoint (Variables|Default|GetPatrolRoute) (Variables|Default|GetpatrolIndex) "World")))