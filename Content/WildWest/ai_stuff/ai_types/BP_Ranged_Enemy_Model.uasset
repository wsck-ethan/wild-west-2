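; Ranged enemy character Blueprint for the WildWest AI that arms itself with a gun.
; BeginPlay runs the parent logic and calls EquipWeopon, spelled differently from the EquipWeapon event defined here.
; The EquipWeapon event spawns BP_gun, snaps it to the mesh's right-hand pistol socket, sets the wielding flag, then calls EquipWeapon.
; Tick, overlap and construction script add no logic of their own.
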(event Custom|Equip%20Weapon
  (bind _returnvalue (Game|SpawnActorfromClass "/Game/WildWest/weopons/BP_gun.BP_gun_C" (Math|Transform|MakeTransform "0, 0, 0") "Undefined" "MultiplyWithRoot" 0 0))
  (bind _output_get (Variables|Default|SetweaponActor _returnvalue))
  (Transformation|AttachComponentToComponent _output_get (Variables|Character|GetMesh) "RHand_Pistol Socket" "SnapToTarget" "SnapToTarget" "SnapToTarget" true)
  (Variables|Default|Setis%20welding%20weopon true)
  (CallFunction|EquipWeapon))

(event EventBeginPlay
  (|CallParentFunction)
  (CallFunction|EquipWeopon))

(event Collision|EventActorBeginOverlap
  (params (OtherActor :type Actor%20Object%20Reference))
  (|CallParentFunction OtherActor) ; This node is disabled and will not be called.\nDrag off pins to build functionality.
)

(event EventTick
  (params (DeltaSeconds :type Float%20%28single-precision%29))
  (|CallParentFunction DeltaSeconds) ; This node is disabled and will not be called.\nDrag off pins to build functionality.
)

(fn ConstructionScript
  (|CallParentFunction))