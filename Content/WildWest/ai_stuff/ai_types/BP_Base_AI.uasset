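; BP_Base_AI is the base AI character for the WildWest game, providing health and shared movement and combat queries.
; Overlaps on its damage collision subtract Health using damage from BP_Projectile_AIDamage and destroy the actor at zero, while other overlaps print a debug "Miss".
; Functions expose fixed attack and defend radii and the patrol route, and map a speed state to the character's max walk speed.
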(event OnComponentBeginOverlap(DamageCollison)
  (params (OverlappedComponent :type Primitive%20Component%20Object%20Reference) (OtherActor :type Actor%20Object%20Reference) (OtherComp :type Primitive%20Component%20Object%20Reference) (OtherBodyIndex :type Integer) (bFromSweep :type Boolean) (SweepResult :type Hit%20Result%20Structure%20%28by%20ref%29))
  (bind _asbp_projectile_aidamage (Utilities|Casting|CastToBP_Projectile_AIDamage OtherActor)
    (:then
      (bind _output_get (Variables|Default|Sethealth (- (Variables|Default|Gethealth) (Variables|/Game/WildWest/Ralph_Young/BP_Projectile_AIDamage.BP_Projectile_AIDamage_C|GetDamage _asbp_projectile_aidamage))))
      (if (<= _output_get 0)
        (Actor|DestroyActor)))
    (:CastFailed
      (Development|PrintString "Miss"))))

(fn ConstructionScript)

(fn Getidealrange
  (return 1.5e+02 3.5e+02))

(fn GetPatrolRoute
  (return (Variables|AI|GetPatrolRoute)))

(fn SetMovementSpeed
  (params (speed :type E_movementSpeed%20Enum :default "NewEnumerator0"))
  (bind _output_get (Variables|/Script/Engine.CharacterMovementComponent|SetMaxWalkSpeed (Variables|Character|GetCharacterMovement) (Utilities|Select :Index speed :NewEnumerator0 0.0 :NewEnumerator1 1e+02 :NewEnumerator2 3e+02 :NewEnumerator3 5e+02)))
  (return _output_get))