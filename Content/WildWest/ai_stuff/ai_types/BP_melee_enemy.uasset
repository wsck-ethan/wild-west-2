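; Melee enemy Blueprint that overrides or handles equip, unequip and attack events through montages on its mesh.
; Montage notifies drive the weapon: "Hold Weopon" spawns a BP_gun on GunSocket, and "Drop Sword" destroys it, each updating the wielding flag.
; Equip and unequip fire dispatcher calls after a short post-montage delay.
; No montage assets are assigned, and Attack only plays a montage and waits, with no damage or completion call.
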(event EventBeginPlay
  (|CallParentFunction))

(event EventEquipWeopon
  (bind _notifyname (Animation|Montage|PlayMontage (Variables|Character|GetMesh) 0)
    (:OnCompleted
      ;[1 1 1] delete when montage play is set
      (Utilities|FlowControl|Delay 1.0)
      (Default|CallOnweoponEquiped))
    (:OnNotifyBegin
      (switch name _notifyname
        (:hold%20weopon
          (bind _returnvalue (Game|SpawnActorfromClass "/Game/WildWest/weopons/BP_gun.BP_gun_C" (Transformation|GetActorTransform) "Undefined" "MultiplyWithRoot" 0 0))
          (bind _output_get (Variables|Default|SetweaponActor _returnvalue))
          (Transformation|AttachComponentToComponent _output_get (Variables|Character|GetMesh) "GunSocket" "SnapToTarget" "SnapToTarget" "SnapToTarget" true)
          (Variables|Default|Setis%20welding%20weopon true))))))

(event EventUnequipWeopon
  (bind _notifyname (Animation|Montage|PlayMontage (Variables|Character|GetMesh) 0)
    (:OnCompleted
      (Utilities|FlowControl|Delay 0.2)
      (Default|CallOnWeoponUnequip))
    (:OnNotifyBegin
      (switch name _notifyname
        (:drop%20sword
          (Actor|DestroyActor (Variables|Default|GetweaponActor))
          (Variables|Default|Setis%20welding%20weopon false))))))

(event EventAttack
  (Animation|Montage|PlayMontage (Variables|Character|GetMesh) 0
    (:OnCompleted
      (Utilities|FlowControl|Delay 0.2))))

(fn ConstructionScript
  (|CallParentFunction))