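; Ranged gun-wielding enemy character that spawns a pistol on BeginPlay and attaches it to its right-hand socket.
; Attack plays a shooting montage; on its notify, a visibility trace runs from gun to the AI controller's target, and an unblocked trace directly subtracts player health.
; Montage completion or interruption signals attack end after a short delay.
; It also supplies movement speeds and ideal attack/defend ranges; its patrol-route getter is empty.
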(event EventBeginPlay
  (|CallParentFunction)
  (CallFunction|EquipWeopon))

(event Collision|EventActorBeginOverlap
  (params (OtherActor :type Actor%20Object%20Reference)))

(event EventTick
  (params (DeltaSeconds :type Float%20%28single-precision%29)))

(event EventEquipWeopon
  (bind _returnvalue (Game|SpawnActorfromClass "/Game/WildWest/weopons/BP_gun.BP_gun_C" (Math|Transform|MakeTransform "0, 0, 0") "Undefined" "MultiplyWithRoot" 0 0))
  (bind _output_get (Variables|Default|SetweaponActor _returnvalue))
  (bind _returnvalue_2 (Transformation|AttachComponentToComponent _output_get (Variables|Character|GetMesh) "RHand_Pistol Socket" "SnapToTarget" "SnapToTarget" "SnapToTarget" true))
  (Variables|Default|Setis%20welding%20weopon _returnvalue_2)
  (Default|CallOnweoponEquiped))

(event EventAttack
  ;[1 1 1] Ai fire animation
  (bind _notifyname (Animation|Montage|PlayMontage (Variables|Character|GetMesh) "/Game/WildWest/Character_s_/Animations/AI_Animations/Montage_Shooting_Gun.Montage_Shooting_Gun")
    (:OnCompleted
      (Utilities|FlowControl|Delay 0.2 :!label _label)
      (Default|CallOnAttackEnd))
    (:OnInterrupted
      (goto _label))
    (:OnNotifyBegin
      (switch name _notifyname
        (:fire
          (bind _asaic_enemy_base (Utilities|Casting|CastToAIC_enemy_base (AI|GetAIController self)))
          (bind _attack_target (Variables|/Game/WildWest/ai_stuff/AIC_enemy_base.AIC_enemy_base_C|GetAttack%20Target _asaic_enemy_base)
            (:then
              (bind _asbp_third_person_character (Utilities|Casting|CastToBP_ThirdPersonCharacter (Game|GetPlayerCharacter 0)))
              (bind _returnvalue (Collision|LineTraceByChannel (Transformation|GetActorLocation (Variables|Default|GetweaponActor)) (Transformation|GetActorLocation _attack_target) "TraceTypeQuery1" false 0 "Persistent"))
              (if (not _returnvalue)
                (Development|PrintString "hit")
                (bind _output_get (Variables|/Game/ThirdPerson/Blueprints/BP_ThirdPersonCharacter.BP_ThirdPersonCharacter_C|SetHealth%203d%20person _asbp_third_person_character (- (Variables|/Game/ThirdPerson/Blueprints/BP_ThirdPersonCharacter.BP_ThirdPersonCharacter_C|GetHealth%203d%20person _asbp_third_person_character) 5)))
                (Development|PrintString (Utilities|String|ToString(Integer) _output_get))))
            (:else)))))))

(fn ConstructionScript
  (|CallParentFunction))

(fn SetMovementSpeed
  (params (speed :type E_movementSpeed%20Enum :default "NewEnumerator0"))
  (bind _output_get (Variables|/Script/Engine.CharacterMovementComponent|SetMaxWalkSpeed (Variables|Character|GetCharacterMovement) (Utilities|Select :Index speed :NewEnumerator0 0.0 :NewEnumerator1 2e+02 :NewEnumerator2 3e+02 :NewEnumerator3 5e+02)))
  (return _output_get))

(fn Getidealrange
  (return 6e+02 6e+02))

(fn GetPatrolRoute
  (return 0))